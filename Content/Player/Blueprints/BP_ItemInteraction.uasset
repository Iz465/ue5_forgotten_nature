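; BP_ItemInteraction is an unfinished item-interaction Blueprint that caches a reference to the player character on BeginPlay.
; A disconnected debug chain would line trace from the player's camera over a grab distance, drawing the trace persistently.
; On hitting a Tools actor, that chain would print the name and damage from its ToolData class defaults.
; Tick is empty, so the trace never runs.
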(event EventBeginPlay
  (bind _asplayer_bp (Utilities|Casting|CastToPlayer_BP (Game|GetPlayerCharacter 0)))
  (Variables|Default|SetAs%20Player%20BP _asplayer_bp))

(event EventTick
  (params (DeltaSeconds :type Float%20%28single-precision%29)))

(event Input|KeyboardEvents|DebugKeyE
  (params (Key :type Key%20Structure :default "None") (ActionValue :type Input%20Action%20Value%20Structure)))